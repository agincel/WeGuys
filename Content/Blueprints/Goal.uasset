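; Level goal actor that loads the next map once both players are on it.
; Overlap events use each character's player index to toggle that player's flag and indicator component, and entries run the Check Load Level check.
; In single player the second player counts as present from the start, otherwise BeginPlay adds the game HUD.
; When both flags are set, it waits briefly, removes the HUD and opens NextMap.
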(event OnComponentBeginOverlap(Goal)
  (params (OtherActor :type Actor%20Object%20Reference) (OtherComp :type Primitive%20Component%20Object%20Reference) (OtherBodyIndex :type Integer) (bFromSweep :type Boolean) (SweepResult :type Hit%20Result%20Structure%20%28by%20ref%29))
  (bind _asmy_character (Utilities|Casting|CastToMyCharacter OtherActor))
  (switch int (Variables|/Game/Blueprints/MyCharacter.MyCharacter_C|GetPlayerIndex _asmy_character)
    (:0
      (Variables|Default|SetP1On true)
      (Components|Activation|SetActive (Variables|Default|GetP1) true false)
      (Utilities|CheckLoadLevel))
    (:1
      (Variables|Default|SetP2On true)
      (Components|Activation|SetActive (Variables|Default|GetP2) true false)
      (Utilities|CheckLoadLevel))))

(event OnComponentEndOverlap(Goal)
  (params (OtherActor :type Actor%20Object%20Reference) (OtherComp :type Primitive%20Component%20Object%20Reference) (OtherBodyIndex :type Integer))
  (bind _asmy_character (Utilities|Casting|CastToMyCharacter OtherActor))
  (switch int (Variables|/Game/Blueprints/MyCharacter.MyCharacter_C|GetPlayerIndex _asmy_character)
    (:0
      (Variables|Default|SetP1On false)
      (Components|Activation|SetActive (Variables|Default|GetP1) false false))
    (:1
      (Variables|Default|SetP2On false)
      (Components|Activation|SetActive (Variables|Default|GetP2) false false))))

(event EventBeginPlay
  (if (Variables|Default|GetisSinglePlayer)
    (Components|Activation|SetActive (Variables|Default|GetP2) true false)
    (Variables|Default|SetP2On true)
    (else
      (bind _returnvalue (UserInterface|CreateWidget "/Game/Blueprints/GameHUD.GameHUD_C"))
      (Variables|Default|SetgameHud _returnvalue)
      (UserInterface|Viewport|AddtoViewport _returnvalue))))

(fn ConstructionScript)