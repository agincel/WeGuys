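; MyPuppeteer is a local two-player controller hub that routes one set of input bindings to two MyCharacter actors.
; On BeginPlay it registers itself with each character, assigns them by PlayerIndex, and raises terminal velocity on every PhysicsVolume.
; Paired inputs forward movement, jump and shoot to each character, while Escape opens the Title level.
; KillAll counts the given player's death, kills both characters and restarts all ambient sounds.
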(event EventBeginPlay
  (bind _outactors (Actor|GetAllActorsOfClass "/Game/Blueprints/MyCharacter.MyCharacter_C"))
  (for _array_element _outactors
    (bind _asmy_character (Utilities|Casting|CastToMyCharacter _array_element))
    (Variables|/Game/Blueprints/MyCharacter.MyCharacter_C|SetOwningPuppeteer _asmy_character self)
    (switch int (Variables|/Game/Blueprints/MyCharacter.MyCharacter_C|GetPlayerIndex _asmy_character)
      (:0
        (Variables|Default|SetPlayer0 _asmy_character))
      (:1
        (Variables|Default|SetPlayer1 _asmy_character))))
  (CallFunction|PhysicsFix))

(event Input|ActionEvents|InputActionJump2
  (:Pressed
    (Default|JumpPressed (Variables|Default|GetPlayer1)))
  (:Released
    (Default|JumpReleased (Variables|Default|GetPlayer1))))

(event Input|ActionEvents|InputActionJump
  (bind _player0 (Variables|Default|GetPlayer0))
  (:Pressed
    (Default|JumpPressed _player0))
  (:Released
    (Default|JumpReleased _player0)))

(event Input|ActionEvents|InputActionShoot
  (:Pressed
    (Default|Shoot (Variables|Default|GetPlayer0))))

(event Input|ActionEvents|InputActionShoot2
  (:Pressed
    (Default|Shoot (Variables|Default|GetPlayer1))))

(event Input|AxisEvents|InputAxisMoveRight2
  (params (AxisValue :type Float%20%28single-precision%29))
  (Default|MyMoveRight (Variables|Default|GetPlayer1) AxisValue))

(event Input|AxisEvents|InputAxisMoveRight
  (params (AxisValue :type Float%20%28single-precision%29))
  (Default|MyMoveRight (Variables|Default|GetPlayer0) AxisValue))

(fn ConstructionScript)

(fn KillAll
  (params (Player%20Index :type Integer))
  (switch int Player%20Index
    (:Default
      _)
    (:0
      (Variables|Default|SetP1Deaths (+ (Variables|Default|GetP1Deaths) 1)))
    (:1
      (Variables|Default|SetP2Deaths (+ (Variables|Default|GetP2Deaths) 1))))
  (Default|Die (Variables|Default|GetPlayer0))
  (Default|Die (Variables|Default|GetPlayer1))
  (bind _outactors (Actor|GetAllActorsOfClass "/Script/Engine.AmbientSound"))
  (for _array_element _outactors
    (Audio|Components|Audio|Stop _array_element)
    (Audio|Components|Audio|Play _array_element 0.0)))

(event Input|ActionEvents|InputActionEscape
  (:Pressed
    (Game|OpenLevel(byName) "Title")))

(fn PhysicsFix
  (bind _outactors (Actor|GetAllActorsOfClass "/Script/Engine.PhysicsVolume"))
  (for _array_element _outactors
    (Variables|/Script/Engine.PhysicsVolume|SetTerminalVelocity _array_element 5e+04)))