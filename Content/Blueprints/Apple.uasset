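; Configurable apple trap that flies toward a destination offset when a MyCharacter enters its trigger zone, killing via the puppeteer's KillAll when the sprite overlaps one.
; BeginPlay applies per-instance trigger placement and scale, debug visibility, sprite, collision and optional material.
; The trigger fires once per life, moving the sprite with one of three speed-selected timelines.
; When movement finishes, it resets and rearms only if Died is set.
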(event OnComponentBeginOverlap(TriggerZone)
  (params (OtherActor :type Actor%20Object%20Reference) (OtherComp :type Primitive%20Component%20Object%20Reference) (OtherBodyIndex :type Integer) (bFromSweep :type Boolean) (SweepResult :type Hit%20Result%20Structure%20%28by%20ref%29))
  (Utilities|Casting|CastToMyCharacter OtherActor)
  (if (not (Variables|Default|GetdidFireThisLife))
    (Variables|Default|Setdied false)
    (Variables|Default|SetdidFireThisLife true)
    (Variables|Default|SetisMoving true)
    (switch Utilities|FlowControl|Switch|SwitchonAppleSpeed (Variables|Default|GetSpeedType)
      (:NewEnumerator0
        (bind _track1 (Timeline|Timeline_0 PlayFromStart)
          (:Update
            (Transformation|SetRelativeLocation (Variables|Default|GetSprite) (Math|Vector|Lerp(Vector) "0, 0, 0" (Variables|Default|GetDestinationOffset) _track1) false))
          (:Finished
            (CallFunction|FinishedTimeline))))
      (:NewEnumerator1
        (bind _track1_2 (Timeline|Timeline_1 PlayFromStart)
          (:Update
            (Transformation|SetRelativeLocation (Variables|Default|GetSprite) (Math|Vector|Lerp(Vector) "0, 0, 0" (Variables|Default|GetDestinationOffset) _track1_2) false))
          (:Finished
            (CallFunction|FinishedTimeline))))
      (:NewEnumerator2
        (bind _track1_3 (Timeline|Timeline_2 PlayFromStart)
          (:Update
            (Transformation|SetRelativeLocation (Variables|Default|GetSprite) (Math|Vector|Lerp(Vector) "0, 0, 0" (Variables|Default|GetDestinationOffset) _track1_3) false))
          (:Finished
            (CallFunction|FinishedTimeline)))))))

(event OnComponentBeginOverlap(Sprite)
  (params (OtherActor :type Actor%20Object%20Reference) (OtherComp :type Primitive%20Component%20Object%20Reference) (OtherBodyIndex :type Integer) (bFromSweep :type Boolean) (SweepResult :type Hit%20Result%20Structure%20%28by%20ref%29))
  (bind _asmy_character (Utilities|Casting|CastToMyCharacter OtherActor))
  (Default|KillAll (Variables|/Game/Blueprints/MyCharacter.MyCharacter_C|GetOwningPuppeteer _asmy_character)))

(event EventBeginPlay
  (bind _debug (Variables|Default|Getdebug))
  ;[1 1 1] Begin Play
  (Transformation|AddLocalOffset (Variables|Default|GetTrigger%20Offset) false)
  (Transformation|SetRelativeScale3D (Variables|Default|GetTriggerZone) (Variables|Default|GetTrigger%20Scale))
  (Rendering|Components|Sprite|SetSprite (Variables|Default|GetSprite) (Variables|Default|GetReplacementSprite))
  (Rendering|SetVisibility _debug (Variables|Default|GetdebugCanSeeTrigger) false)
  (Transformation|SetWorldScale3D _debug (/ (Variables|Default|GetTrigger%20Scale) 3.0))
  (Collision|SetCollisionResponsetoAllChannels (Variables|Default|GetSprite) (Variables|Default|GetCollisionType))
  (Transformation|SetRelativeScale3D (Variables|Default|GetSprite) (Variables|Default|GetAppleScale))
  (if (Variables|Default|GetuseMaterial)
    (Rendering|Material|SetMaterial (Variables|Default|GetSprite) 0 (Variables|Default|GetReplacementMaterial))))

(fn ConstructionScript)

(fn FinishedTimeline
  (Variables|Default|SetisMoving false)
  (if (Variables|Default|Getdied)
    (Transformation|SetRelativeLocation (Variables|Default|GetSprite) "0, 0, 0" false)
    (Variables|Default|Setdied false)
    (Variables|Default|SetdidFireThisLife false))
  (return))