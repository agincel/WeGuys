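; PlayerGate is a trigger gate that lets only the character with a matching player index pass.
; At BeginPlay it copies AllowedIndex into IndexOverride and shows that number, one-based, on the Indicator text.
; The Override event swaps the active index and updates the text at runtime.
; When a MyCharacter with a different index overlaps the Gate, its OwningPuppeteer calls KillAll with that character's index.
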(event OnComponentBeginOverlap(Gate)
  (params (OtherActor :type Actor%20Object%20Reference) (OtherComp :type Primitive%20Component%20Object%20Reference) (OtherBodyIndex :type Integer) (bFromSweep :type Boolean) (SweepResult :type Hit%20Result%20Structure%20%28by%20ref%29))
  (bind _asmy_character (Utilities|Casting|CastToMyCharacter OtherActor))
  (if (not (== (Variables|Default|GetIndexOverride) (Variables|/Game/Blueprints/MyCharacter.MyCharacter_C|GetPlayerIndex _asmy_character)))
    (Default|KillAll (Variables|/Game/Blueprints/MyCharacter.MyCharacter_C|GetOwningPuppeteer _asmy_character) (Variables|/Game/Blueprints/MyCharacter.MyCharacter_C|GetPlayerIndex _asmy_character))))

(event Custom|Initialize
  (bind _allowedindex (Variables|Default|GetAllowedIndex))
  (Rendering|Components|TextRender|SetText (Variables|Default|GetIndicator) (Utilities|String|ToString(Integer) (+ _allowedindex 1)))
  (Variables|Default|SetIndexOverride _allowedindex))

(event Custom|Override
  (params (New%20Index :type Integer))
  (Variables|Default|SetIndexOverride New%20Index)
  (Rendering|Components|TextRender|SetText (Variables|Default|GetIndicator) (Utilities|String|ToString(Integer) (+ New%20Index 1))))

(event EventBeginPlay
  (CallFunction|Initialize))

(fn ConstructionScript)