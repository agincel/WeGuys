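; Moving platform, apparently Paper2D, that shuttles endlessly between its origin and DestinationOffset.
; BeginPlay picks one of three timelines from the Speed setting, Fast, Medium or Slow, each driving a relative-location lerp without sweep.
; Each timeline reverses at either end to ping-pong, and a set Died flag is cleared on the next update and restarts the motion from the start.
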(event EventBeginPlay
  (switch Utilities|FlowControl|Switch|SwitchonAppleSpeed (Variables|Default|GetSpeed)
    (:NewEnumerator0
      (bind (_direction _track1) (Timeline|Translate PlayFromStart)
        (:Update
          (if (Variables|Default|Getdied)
            (Variables|Default|Setdied false)
            (Timeline|Translate PlayFromStart)
            (else
              (Transformation|SetRelativeLocation (Math|Vector|Lerp(Vector) "0, 0, 0" (Variables|Default|GetDestinationOffset) _track1) false))))
        (:Finished
          (switch Utilities|FlowControl|Switch|SwitchonETimelineDirection _direction
            (:Forward
              (Timeline|Translate Reverse))
            (:Backward
              (Timeline|Translate Play))))))
    (:NewEnumerator1
      (bind (_direction_2 _track1_2) (Timeline|Timeline_0 PlayFromStart)
        (:Update
          (if (Variables|Default|Getdied)
            (Variables|Default|Setdied false)
            (Timeline|Timeline_0 PlayFromStart)
            (else
              (Transformation|SetRelativeLocation (Variables|Default|GetPaperSprite1) (Math|Vector|Lerp(Vector) "0, 0, 0" (Variables|Default|GetDestinationOffset) _track1_2) false))))
        (:Finished
          (switch Utilities|FlowControl|Switch|SwitchonETimelineDirection _direction_2
            (:Forward
              (Timeline|Timeline_0 Reverse))
            (:Backward
              (Timeline|Timeline_0 Play))))))
    (:NewEnumerator2
      (bind (_direction_3 _track1_3) (Timeline|Timeline_1 PlayFromStart)
        (:Update
          (if (Variables|Default|Getdied)
            (Variables|Default|Setdied false)
            (Timeline|Timeline_1 PlayFromStart)
            (else
              (Transformation|SetRelativeLocation (Variables|Default|GetPaperSprite1) (Math|Vector|Lerp(Vector) "0, 0, 0" (Variables|Default|GetDestinationOffset) _track1_3) false))))
        (:Finished
          (switch Utilities|FlowControl|Switch|SwitchonETimelineDirection _direction_3
            (:Forward
              (Timeline|Timeline_1 Reverse))
            (:Backward
              (Timeline|Timeline_1 Play))))))))

(fn ConstructionScript)