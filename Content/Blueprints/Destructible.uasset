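; Destructible actor that takes damage from Bullet overlaps and disappears once its health runs out.
; Each hit spawns a bullet-hit particle effect, calls the bullet's DestroySelf and removes one point of health, which starts at InitialHealth.
; DestroySelf only hides the component and disables its collision instead of destroying the actor, so RecreateSelf can restore visibility, collision and full health.
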(event OnComponentBeginOverlap(Destructable)
  (params (OtherActor :type Actor%20Object%20Reference) (OtherComp :type Primitive%20Component%20Object%20Reference) (OtherBodyIndex :type Integer) (bFromSweep :type Boolean) (SweepResult :type Hit%20Result%20Structure%20%28by%20ref%29))
  (bind _asbullet (Utilities|Casting|CastToBullet OtherActor))
  (Effects|SpawnEmitteratLocation "/Game/StarterContent/Particles/P_BulletHit.P_BulletHit" (Transformation|GetActorLocation _asbullet))
  (Default|DestroySelf _asbullet)
  (Variables|Default|SetHealth (- (Variables|Default|GetHealth) 1))
  (if (== (Variables|Default|GetHealth) 0)
    (CallFunction|DestroySelf)))

(event EventBeginPlay
  (Variables|Default|SetHealth (Variables|Default|GetinitialHealth)))

(fn ConstructionScript)

(fn DestroySelf
  (Collision|SetCollisionEnabled (Variables|Default|GetDestructable) "NoCollision")
  (Rendering|SetVisibility (Variables|Default|GetDestructable) false false))

(fn RecreateSelf
  (Collision|SetCollisionEnabled (Variables|Default|GetDestructable) "QueryAndPhysics")
  (Rendering|SetVisibility (Variables|Default|GetDestructable) true false)
  (Variables|Default|SetHealth (Variables|Default|GetinitialHealth)))