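; Portal actor with linked Blue and Orange ends that teleports MyCharacter from whichever it overlaps to the other.
; BeginPlay applies the configured offset and rotations, and each teleport rotates velocity by the combined portal rotators and re-enables double jump.
; Only Blue-to-Orange caps X velocity at max walk speed, zeroing Y when capped.
; Passing-through flags, cleared on end overlap at the exit, prevent immediate bounce-back.
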(event OnComponentBeginOverlap(Blue)
  (params (OtherActor :type Actor%20Object%20Reference) (OtherComp :type Primitive%20Component%20Object%20Reference) (OtherBodyIndex :type Integer) (bFromSweep :type Boolean) (SweepResult :type Hit%20Result%20Structure%20%28by%20ref%29))
  (if (not (Variables|Default|GetpassingThroughOrange))
    (Variables|Default|SetpassingThroughBlue true)
    (bind _asmy_character (Utilities|Casting|CastToMyCharacter OtherActor))
    (Transformation|SetActorLocation _asmy_character (Transformation|GetWorldLocation (Variables|Default|GetOrange)) false)
    (if (< (.X (Math|Vector|BreakVector (Math|Vector|RotateVector (Transformation|GetVelocity _asmy_character) (Math|Rotator|CombineRotators (Variables|Default|GetBlueRotator) (* (Variables|Default|GetOrangeRotator) -1.0))))) (Variables|/Script/Engine.CharacterMovementComponent|GetMaxWalkSpeed (Variables|/Script/Engine.Character|GetCharacterMovement _asmy_character)))
      (Variables|/Script/Engine.MovementComponent|SetVelocity (Variables|/Script/Engine.Character|GetCharacterMovement _asmy_character) (Math|Vector|RotateVector (Transformation|GetVelocity _asmy_character) (Math|Rotator|CombineRotators (Variables|Default|GetBlueRotator) (* (Variables|Default|GetOrangeRotator) -1.0))))
      (else
        (Variables|/Script/Engine.MovementComponent|SetVelocity (Variables|/Script/Engine.Character|GetCharacterMovement _asmy_character) (Math|Vector|MakeVector (Variables|/Script/Engine.CharacterMovementComponent|GetMaxWalkSpeed (Variables|/Script/Engine.Character|GetCharacterMovement _asmy_character)) 0.0 (.Z (Math|Vector|BreakVector (Math|Vector|RotateVector (Transformation|GetVelocity _asmy_character) (Math|Rotator|CombineRotators (Variables|Default|GetBlueRotator) (* (Variables|Default|GetOrangeRotator) -1.0)))))))))
    (Variables|/Game/Blueprints/MyCharacter.MyCharacter_C|SetcanDoubleJump _asmy_character true)))

(event OnComponentBeginOverlap(Orange)
  (params (OtherActor :type Actor%20Object%20Reference) (OtherComp :type Primitive%20Component%20Object%20Reference) (OtherBodyIndex :type Integer) (bFromSweep :type Boolean) (SweepResult :type Hit%20Result%20Structure%20%28by%20ref%29))
  (if (not (Variables|Default|GetpassingThroughBlue))
    (Variables|Default|SetpassingThroughOrange true)
    (bind _asmy_character (Utilities|Casting|CastToMyCharacter OtherActor))
    (Transformation|SetActorLocation _asmy_character (Transformation|GetWorldLocation (Variables|Default|GetBlue)) false)
    (Variables|/Script/Engine.MovementComponent|SetVelocity (Variables|/Script/Engine.Character|GetCharacterMovement _asmy_character) (Math|Vector|RotateVector (Transformation|GetVelocity _asmy_character) (Math|Rotator|CombineRotators (Variables|Default|GetBlueRotator) (* (Variables|Default|GetOrangeRotator) -1.0))))
    (Variables|/Game/Blueprints/MyCharacter.MyCharacter_C|SetcanDoubleJump _asmy_character true)))

(event OnComponentEndOverlap(Blue)
  (params (OtherActor :type Actor%20Object%20Reference) (OtherComp :type Primitive%20Component%20Object%20Reference) (OtherBodyIndex :type Integer))
  (Utilities|Casting|CastToMyCharacter OtherActor)
  (Variables|Default|SetpassingThroughOrange false))

(event OnComponentEndOverlap(Orange)
  (params (OtherActor :type Actor%20Object%20Reference) (OtherComp :type Primitive%20Component%20Object%20Reference) (OtherBodyIndex :type Integer))
  (Utilities|Casting|CastToMyCharacter OtherActor)
  (Variables|Default|SetpassingThroughBlue false))

(event EventBeginPlay
  (Transformation|AddLocalOffset (Variables|Default|GetOrange) (Variables|Default|GetOrangeOffset) false)
  (Transformation|AddLocalRotation (Variables|Default|GetOrange) (Variables|Default|GetOrangeRotator) false)
  (Transformation|AddLocalRotation (Variables|Default|GetBlue) (Variables|Default|GetBlueRotator) false)
  (Variables|Default|SetpassingThroughBlue false)
  (Variables|Default|SetpassingThroughOrange false))

(fn ConstructionScript)