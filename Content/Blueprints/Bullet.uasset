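; Projectile actor fired by a character that kills other characters it overlaps.
; Define flips the speed for left-facing shots, increments the owner's bullet count and starts the bullet, which then moves every Tick without sweeping.
; Overlapping another MyCharacter calls KillAll on its puppeteer without destroying the bullet.
; Apples and the owner are ignored; any other overlap destroys the bullet and decrements the count.
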(event OnComponentBeginOverlap(Bullet)
  (params (OtherActor :type Actor%20Object%20Reference) (OtherComp :type Primitive%20Component%20Object%20Reference) (OtherBodyIndex :type Integer) (bFromSweep :type Boolean) (SweepResult :type Hit%20Result%20Structure%20%28by%20ref%29))
  (if (Variables|Default|GethasStarted)
    (bind _asmy_character (Utilities|Casting|CastToMyCharacter OtherActor)
      (:then
        (if (not (== (Variables|Default|GetOwningCharacter) OtherActor))
          (Default|KillAll (Variables|/Game/Blueprints/MyCharacter.MyCharacter_C|GetOwningPuppeteer _asmy_character))))
      (:CastFailed
        (Utilities|Casting|CastToApple OtherActor
          (:CastFailed
            (CallFunction|DestroySelf)))))))

(event Custom|Define
  (params (isFacingRight :type Boolean))
  (bind _owningcharacter (Variables|Default|GetOwningCharacter))
  (if isFacingRight
    _
    (else
      (Variables|Default|SetSpeed (* (Variables|Default|GetSpeed) -1.0))))
  (Variables|/Game/Blueprints/MyCharacter.MyCharacter_C|SetnumBullets _owningcharacter (+ (Variables|/Game/Blueprints/MyCharacter.MyCharacter_C|GetnumBullets _owningcharacter) 1))
  (Variables|Default|SethasStarted true))

(event EventTick
  (params (DeltaSeconds :type Float%20%28single-precision%29))
  (if (Variables|Default|GethasStarted)
    (Transformation|AddActorWorldOffset (* (Variables|Default|GetSpeed) DeltaSeconds))))

(fn ConstructionScript)

(fn DestroySelf
  (bind _owningcharacter (Variables|Default|GetOwningCharacter))
  (Variables|/Game/Blueprints/MyCharacter.MyCharacter_C|SetnumBullets _owningcharacter (- (Variables|/Game/Blueprints/MyCharacter.MyCharacter_C|GetnumBullets _owningcharacter) 1))
  (Actor|DestroyActor))